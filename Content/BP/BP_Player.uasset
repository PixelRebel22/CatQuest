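; Player character with Enhanced Input movement, look, sprint and jump, plus ledge mantling and a death event that reloads CatQuest.
; Jump calls TryMantle, which chains forward, vertical and ground line traces with height limits to set the mantle target.
; A timeline then moves the character in Flying mode along an arced, swept lerp, aborting when the move returns true.
; Debug prints and draws remain; the capsule clearance check is unconnected.
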(event Custom|KillPlayer
  (params (Player :type Actor%20Object%20Reference))
  ;[0.15 0.15 0.15 0.5] Kill Player
  (Input|DisableInput Player (Game|GetPlayerController 0))
  (Utilities|FlowControl|Delay 0.5)
  (Game|OpenLevel(byName) "CatQuest"))

(event Custom|PlayMantleTimeline
  (Variables|Default|SetbIsMantling true)
  (Pawn|Components|CharacterMovement|SetMovementMode (Variables|Character|GetCharacterMovement) "MOVE_Flying" 0)
  (Utilities|FlowControl|Sequence
    (:then_0
      (bind (_direction _alpha _arc) (Timeline|Timeline_Mantle SetNewTime)
        (:Update
          (Development|PrintString (Utilities|String|Append "Arc= " (Utilities|String|ToString(Float) _arc)))
          (Development|PrintString (Utilities|String|Append "LiftZ= " (Utilities|String|ToString(Float) (.Z (Math|Vector|BreakVector (* (* (Variables|Default|GetArcHeight) _arc) (Math|Vector|GetUpVector "0, 0, 0")))))))
          (Development|PrintString (Utilities|String|Append "Alpha= " (Utilities|String|ToString(Float) _alpha)))
          (bind _returnvalue (Transformation|SetActorLocationAndRotation (+ (Math|Vector|Lerp(Vector) (Variables|Default|GetMantleStartLocation) (Variables|Default|GetMantleTargetLocation) _alpha) (* (* (Variables|Default|GetArcHeight) _arc) (Math|Vector|GetUpVector "0, 0, 0"))) (Math|Interpolation|RInterpTo (Transformation|GetActorRotation) (Variables|Default|GetMantleTargetRotation) (Utilities|Time|GetWorldDeltaSeconds) (Variables|Default|GetMantleLerpSpeedRot)) true))
          (if _returnvalue
            (CallFunction|AbortMantle)
            (else
              (Development|PrintString "In the middle of mantling"))))
        (:Finished
          (Variables|Default|SetbIsMantling false)
          (Pawn|Components|CharacterMovement|SetMovementMode (Variables|Character|GetCharacterMovement) "MOVE_Walking" 0)
          (Development|PrintString "Mantled!"))))
    (:then_1
      (Timeline|Timeline_Mantle PlayFromStart))))

(event Custom|AbortMantle
  (Variables|Default|SetbIsMantling false)
  (Pawn|Components|CharacterMovement|SetMovementMode (Variables|Character|GetCharacterMovement) "MOVE_Walking" 0)
  (Development|PrintString "Mantle ABORT")
  (bind (_direction _alpha _arc) (Timeline|Timeline_Mantle Stop)
    (:Update
      (Development|PrintString (Utilities|String|Append "Arc= " (Utilities|String|ToString(Float) _arc)))
      (Development|PrintString (Utilities|String|Append "LiftZ= " (Utilities|String|ToString(Float) (.Z (Math|Vector|BreakVector (* (* (Variables|Default|GetArcHeight) _arc) (Math|Vector|GetUpVector "0, 0, 0")))))))
      (Development|PrintString (Utilities|String|Append "Alpha= " (Utilities|String|ToString(Float) _alpha)))
      (bind _returnvalue (Transformation|SetActorLocationAndRotation (+ (Math|Vector|Lerp(Vector) (Variables|Default|GetMantleStartLocation) (Variables|Default|GetMantleTargetLocation) _alpha) (* (* (Variables|Default|GetArcHeight) _arc) (Math|Vector|GetUpVector "0, 0, 0"))) (Math|Interpolation|RInterpTo (Transformation|GetActorRotation) (Variables|Default|GetMantleTargetRotation) (Utilities|Time|GetWorldDeltaSeconds) (Variables|Default|GetMantleLerpSpeedRot)) true))
      (if _returnvalue
        (CallFunction|AbortMantle)
        (else
          (Development|PrintString "In the middle of mantling"))))
    (:Finished
      (Variables|Default|SetbIsMantling false)
      (Pawn|Components|CharacterMovement|SetMovementMode (Variables|Character|GetCharacterMovement) "MOVE_Walking" 0)
      (Development|PrintString "Mantled!"))))

(event Input|EnhancedActionEvents|EnhancedInputActionIA_Locomotion
  (params (ActionValue :type Float%20%28double-precision%29) (ElapsedSeconds :type Float%20%28double-precision%29) (TriggeredSeconds :type Float%20%28double-precision%29) (InputAction :type Input%20Action%20Object%20Reference :default "/Game/BP/IO/IA_Locomotion.IA_Locomotion"))
  ;[0.15 0.15 0.15 0.5] Movement Mapping
  (Pawn|Input|AddMovementInput (Transformation|GetActorForwardVector) ActionValue false))

(event Input|EnhancedActionEvents|EnhancedInputActionIA_Strafe
  (params (ActionValue :type Float%20%28double-precision%29) (ElapsedSeconds :type Float%20%28double-precision%29) (TriggeredSeconds :type Float%20%28double-precision%29) (InputAction :type Input%20Action%20Object%20Reference :default "/Game/BP/IO/IA_Strafe.IA_Strafe"))
  ;[0.15 0.15 0.15 0.5] Movement Mapping
  (Pawn|Input|AddMovementInput (Transformation|GetActorRightVector) ActionValue false))

(event Input|EnhancedActionEvents|EnhancedInputActionIA_LookV
  (params (ActionValue :type Float%20%28double-precision%29) (ElapsedSeconds :type Float%20%28double-precision%29) (TriggeredSeconds :type Float%20%28double-precision%29) (InputAction :type Input%20Action%20Object%20Reference :default "/Game/BP/IO/IA_LookV.IA_LookV"))
  ;[0.15 0.15 0.15 0.5] Movement Mapping
  (Pawn|Input|AddControllerPitchInput ActionValue))

(event Input|EnhancedActionEvents|EnhancedInputActionIA_LookH
  (params (ActionValue :type Float%20%28double-precision%29) (ElapsedSeconds :type Float%20%28double-precision%29) (TriggeredSeconds :type Float%20%28double-precision%29) (InputAction :type Input%20Action%20Object%20Reference :default "/Game/BP/IO/IA_LookH.IA_LookH"))
  ;[0.15 0.15 0.15 0.5] Movement Mapping
  (Pawn|Input|AddControllerYawInput ActionValue))

(event Input|EnhancedActionEvents|EnhancedInputActionIA_Jump
  (params (ActionValue :type Float%20%28double-precision%29) (ElapsedSeconds :type Float%20%28double-precision%29) (TriggeredSeconds :type Float%20%28double-precision%29) (InputAction :type Input%20Action%20Object%20Reference :default "/Game/BP/IO/IA_Jump.IA_Jump"))
  ;[0.15 0.15 0.15 0.5] Movement Mapping
  (:Triggered
    (Character|Jump)
    (if (not (Variables|Default|GetbIsMantling))
      (Development|PrintString "Jump pressed")
      (CallFunction|TryMantle)))
  (:Completed
    (Character|StopJumping)))

(event Input|EnhancedActionEvents|EnhancedInputActionIA_Sprint
  (params (ActionValue :type Float%20%28double-precision%29) (ElapsedSeconds :type Float%20%28double-precision%29) (TriggeredSeconds :type Float%20%28double-precision%29) (InputAction :type Input%20Action%20Object%20Reference :default "/Game/BP/IO/IA_Sprint.IA_Sprint"))
  ;[0.15 0.15 0.15 0.5] Movement Mapping
  (:Started
    (Variables|/Script/Engine.CharacterMovementComponent|SetMaxWalkSpeed (Variables|Character|GetCharacterMovement) 5e+02))
  (:Completed
    (Variables|/Script/Engine.CharacterMovementComponent|SetMaxWalkSpeed (Variables|Character|GetCharacterMovement) 4e+02)))

(event EventBeginPlay
  ;[0.15 0.15 0.15 0.5] Establish IMC Mapping
  (Input|AddMappingContext (PlayerController|LocalPlayerSubsystems|GetEnhancedInputLocalPlayerSubsystem (Game|GetPlayerController 0)) "/Game/BP/IO/IMC_Player.IMC_Player" 0 "(bIgnoreAllPressedKeysUntilRelease=True,bForceImmediately=False,bNotifyUserSettings=False)")
  (Variables|Default|SetCapsuleHalfHeight (Components|Capsule|GetScaledCapsuleHalfHeight (Variables|Collision|GetCapsuleComponent))))

(fn ConstructionScript)

(fn TryMantle
  (bind _returnvalue (Transformation|GetActorForwardVector))
  (bind _returnvalue_2 (Math|Vector|GetUpVector "0.000000,1.000000,0.000000"))
  (bind _returnvalue_3 (Math|Vector|ProjectVectorontoPlane _returnvalue _returnvalue_2))
  (bind _returnvalue_4 (Math|Vector|Normalize _returnvalue_3))
  (bind _output_get (LocalVariables|SetTraceStart (+ (+ (Transformation|GetActorLocation) (* (Transformation|GetActorForwardVector) (Math|Float|MakeLiteralFloat 2e+01))) (Math|Vector|MakeVector 0.0 0.0 1e+01))))
  (bind (_outhit _returnvalue_5) (Collision|LineTraceByChannel _output_get (+ (LocalVariables|GetTraceStart) (* (Transformation|GetActorForwardVector) (Variables|Default|GetForwardProbeDistance))) "TraceTypeQuery1" false 0 "ForDuration")) ; ForwardTrace
  (if _returnvalue_5
    (Development|PrintString "Passed forward trace" true true "(R=0.598860,G=0.096443,B=1.000000,A=1.000000)")
    (bind _result (Math|Float|NegateFloat (* (Variables|Default|GetUpProbeHeight) (Math|Float|MakeLiteralFloat 1.25)))
      (:%20%20
        (bind _outhit_2 (Collision|LineTraceByChannel (+ (- (.ImpactPoint (Collision|BreakHitResult _outhit)) (* (.ImpactNormal (Collision|BreakHitResult _outhit)) (Math|Float|MakeLiteralFloat 8.0))) (Variables|Default|GetUpProbeHeight)) (+ (+ (- (.ImpactPoint (Collision|BreakHitResult _outhit)) (* (.ImpactNormal (Collision|BreakHitResult _outhit)) (Math|Float|MakeLiteralFloat 8.0))) (Variables|Default|GetUpProbeHeight)) _result) "TraceTypeQuery1" false 0 "ForDuration")) ; UpTrace
        (Development|PrintString "Passed up trace" true true "(R=0.106316,G=0.439087,B=1.000000,A=1.000000)")
        (if (>= (- (.z (.ImpactPoint (Collision|BreakHitResult _outhit_2))) (- (.z (Transformation|GetActorLocation)) (Variables|Default|GetCapsuleHalfHeight))) (Variables|Default|GetMinMantleHeight))
          (Variables|Default|SetHeight (- (.z (.ImpactPoint (Collision|BreakHitResult _outhit_2))) (- (.z (Transformation|GetActorLocation)) (Variables|Default|GetCapsuleHalfHeight))))
          (Variables|Default|SetFinalForward _returnvalue_4)
          (Development|PrintString "Passed first branch" true true "(R=1.000000,G=0.036059,B=0.076657,A=1.000000)")
          (if (<= (- (.z (.ImpactPoint (Collision|BreakHitResult _outhit_2))) (- (.z (Transformation|GetActorLocation)) (Variables|Default|GetCapsuleHalfHeight))) (Variables|Default|GetMaxMantleHeight))
            (Development|PrintString "passed second branch" true true "(R=1.000000,G=0.582146,B=0.088154,A=1.000000)")
            (bind (_outhit_3 _returnvalue_6) (Collision|LineTraceByChannel (- (.ImpactPoint (Collision|BreakHitResult _outhit_2)) (* _returnvalue_4 (Variables|Default|GetLedgePadding))) "0, 0, 0" "TraceTypeQuery1" false 0 "ForDuration")) ; GroundTrace
            (if _returnvalue_6
              (Development|PrintString "Passed ground trace" true true "(R=0.109375,G=0.055241,B=0.006528,A=1.000000)")
              (Variables|Default|SetMantleTargetLocation (+ (* (Variables|Default|GetFinalForward) (Variables|Default|GetLedgePadding)) (.ImpactPoint (Collision|BreakHitResult _outhit_3))))
              (Variables|Default|SetMantleTargetRotation (Math|Rotator|MakeRotfromX (Variables|Default|GetFinalForward)))
              (Variables|Default|SetMantleStartLocation (- (Transformation|GetActorLocation) (* (Variables|Default|GetFinalForward) (Math|Float|MakeLiteralFloat 2.0))))
              (Variables|Default|SetArcHeight (Math|Float|Clamp(Float) (* (Variables|Default|GetHeight) 0.6) 12.0 3e+01))
              (Rendering|Debug|DrawDebugSphere (Variables|Default|GetMantleTargetLocation) 15.0 12 "(R=0.055248,G=0.000000,B=1.000000,A=1.000000)" 0.0 1.0)
              (CallFunction|PlayMantleTimeline))))))))