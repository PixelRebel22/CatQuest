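; Player character Blueprint with Enhanced Input movement, look, sprint, jump, mantling and a timed attack, plus a death event that opens CatQuest.
; Holding jump while airborne polls camera line and sphere traces for a clear ledge, then a timeline lerps the actor up.
; Attack opens a timing window shown by WBP_TimingRing; later presses print Early, Good, Perfect or Miss.
; Only timer expiry clears timing mode, printing Miss and starting cooldown.
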(event Custom|KillPlayer
  (params (Player :type Actor%20Object%20Reference))
  ;[0.15 0.15 0.15 0.5] Kill Player
  (Input|DisableInput Player (Game|GetPlayerController 0))
  (Utilities|FlowControl|Delay 0.5)
  (Game|OpenLevel(byName) "CatQuest"))

(event Custom|EstablishIMC
  ;[0.15 0.15 0.15 0.5] Establish IMC Mapping
  (Input|AddMappingContext (PlayerController|LocalPlayerSubsystems|GetEnhancedInputLocalPlayerSubsystem (Game|GetPlayerController 0)) "/Game/BP/IO/IMC_Player.IMC_Player" 0 "(bIgnoreAllPressedKeysUntilRelease=True,bForceImmediately=False,bNotifyUserSettings=False)"))

(event Custom|Widget
  (if (not (Utilities|IsValid (Variables|Default|GetTimingWidget)))
    (bind _returnvalue (UserInterface|CreateWidget "/Game/BP/TimedAttack/WBP_TimingRing.WBP_TimingRing_C" (Game|GetPlayerController 0)))
    (bind _output_get (Variables|Default|SetTimingWidget _returnvalue))
    (UserInterface|Viewport|AddtoViewport _output_get 1000)
    (Widget|SetVisibility _output_get "Hidden")))

(event Custom|MantleUp
  ;[0.15 0.15 0.15 0.5] Mantle Timeline
  (Variables|Default|SetbHitDetected false)
  (bind _alpha (Timeline|Mantle PlayFromStart)
    (:Update
      (Transformation|SetActorLocation (Math|Vector|Lerp(Vector) (Transformation|GetActorLocation) (Variables|Default|GetVector) _alpha) false false))))

(event Custom|HandleAttackInput
  ;[0.15 0.15 0.15 0.5] TimedAttack
  (bind _output_get (Variables|Default|SetPressedAt (Utilities|Time|GetGameTimeinSeconds)))
  (if (Variables|Default|GetbInTimingMode)
    (CallFunction|ResolveTiming _output_get)
    (else
      (CallFunction|StartTiming))))

(event Custom|Timer
  (bind _config (Variables|Default|GetConfig))
  ;[0.15 0.15 0.15 0.5] TimedAttack
  (Utilities|Time|SetTimerbyEvent (delegate Custom|Timer%20Expired) (+ (.opendelay _config) (.windowlength _config) (.lategrace _config))))

(event Custom|Timer%20Expired
  ;[0.15 0.15 0.15 0.5] TimedAttack
  (CallFunction|EndTiming true))

(event Input|EnhancedActionEvents|EnhancedInputActionIA_Locomotion
  (params (ActionValue :type Float%20%28double-precision%29) (ElapsedSeconds :type Float%20%28double-precision%29) (TriggeredSeconds :type Float%20%28double-precision%29) (InputAction :type Input%20Action%20Object%20Reference :default "/Game/BP/IO/IA_Locomotion.IA_Locomotion"))
  ;[0.15 0.15 0.15 0.5] Movement Mapping
  (Pawn|Input|AddMovementInput (Transformation|GetActorForwardVector) ActionValue false))

(event Input|EnhancedActionEvents|EnhancedInputActionIA_Strafe
  (params (ActionValue :type Float%20%28double-precision%29) (ElapsedSeconds :type Float%20%28double-precision%29) (TriggeredSeconds :type Float%20%28double-precision%29) (InputAction :type Input%20Action%20Object%20Reference :default "/Game/BP/IO/IA_Strafe.IA_Strafe"))
  ;[0.15 0.15 0.15 0.5] Movement Mapping
  (Pawn|Input|AddMovementInput (Transformation|GetActorRightVector) ActionValue false))

(event Input|EnhancedActionEvents|EnhancedInputActionIA_LookV
  (params (ActionValue :type Float%20%28double-precision%29) (ElapsedSeconds :type Float%20%28double-precision%29) (TriggeredSeconds :type Float%20%28double-precision%29) (InputAction :type Input%20Action%20Object%20Reference :default "/Game/BP/IO/IA_LookV.IA_LookV"))
  ;[0.15 0.15 0.15 0.5] Movement Mapping
  (Pawn|Input|AddControllerPitchInput ActionValue))

(event Input|EnhancedActionEvents|EnhancedInputActionIA_LookH
  (params (ActionValue :type Float%20%28double-precision%29) (ElapsedSeconds :type Float%20%28double-precision%29) (TriggeredSeconds :type Float%20%28double-precision%29) (InputAction :type Input%20Action%20Object%20Reference :default "/Game/BP/IO/IA_LookH.IA_LookH"))
  ;[0.15 0.15 0.15 0.5] Movement Mapping
  (Pawn|Input|AddControllerYawInput ActionValue))

(event Input|EnhancedActionEvents|EnhancedInputActionIA_Jump
  (params (ActionValue :type Float%20%28double-precision%29) (ElapsedSeconds :type Float%20%28double-precision%29) (TriggeredSeconds :type Float%20%28double-precision%29) (InputAction :type Input%20Action%20Object%20Reference :default "/Game/BP/IO/IA_Jump.IA_Jump"))
  ;[0.15 0.15 0.15 0.5] Movement Mapping
  (:Triggered
    ;[0.15 0.15 0.15 0.5] Mantle
    (if (AI|Components|NavMovement|IsFalling (Variables|Character|GetCharacterMovement))
      (bind _output_get (Variables|Default|SetbHeld true))
      (if (and _output_get (AI|Components|NavMovement|IsFalling (Variables|Character|GetCharacterMovement))) :!label _label
        (if (Variables|Default|GetbHitDetected)
          (CallFunction|MantleUp)
          (else
            (CallFunction|MantleCheck)
            (Utilities|FlowControl|Delay 0.01)
            (goto _label))))
      (else
        (Character|Jump))))
  (:Completed
    (Character|StopJumping)
    (Variables|Default|SetbHeld false)))

(event Input|EnhancedActionEvents|EnhancedInputActionIA_Sprint
  (params (ActionValue :type Float%20%28double-precision%29) (ElapsedSeconds :type Float%20%28double-precision%29) (TriggeredSeconds :type Float%20%28double-precision%29) (InputAction :type Input%20Action%20Object%20Reference :default "/Game/BP/IO/IA_Sprint.IA_Sprint"))
  ;[0.15 0.15 0.15 0.5] Movement Mapping
  (:Started
    (Variables|/Script/Engine.CharacterMovementComponent|SetMaxWalkSpeed (Variables|Character|GetCharacterMovement) 5e+02))
  (:Completed
    (Variables|/Script/Engine.CharacterMovementComponent|SetMaxWalkSpeed (Variables|Character|GetCharacterMovement) 4e+02)))

(event Input|EnhancedActionEvents|EnhancedInputActionIA_Attack
  (params (ActionValue :type Float%20%28double-precision%29) (ElapsedSeconds :type Float%20%28double-precision%29) (TriggeredSeconds :type Float%20%28double-precision%29) (InputAction :type Input%20Action%20Object%20Reference :default "/Game/BP/IO/IA_Attack.IA_Attack"))
  ;[0.15 0.15 0.15 0.5] Movement Mapping
  (:Started
    (CallFunction|HandleAttackInput)))

(event EventTick
  (params (DeltaSeconds :type Float%20%28single-precision%29))
  (if (Variables|Default|GetbShowTimingUI)
    (Default|SetPercent (Variables|Default|GetTimingWidget) (Math|Float|Clamp(Float) (/ (- (Utilities|Time|GetGameTimeinSeconds) (Variables|Default|GetWindowOpensAt)) (- (Variables|Default|GetWindowClosesAt) (Variables|Default|GetWindowOpensAt)))) (/ (- (Variables|Default|GetPerfectStart) (Variables|Default|GetWindowOpensAt)) (- (Variables|Default|GetWindowClosesAt) (Variables|Default|GetWindowOpensAt))) (/ (- (Variables|Default|GetPerfectEnd) (Variables|Default|GetWindowOpensAt)) (- (Variables|Default|GetWindowClosesAt) (Variables|Default|GetWindowOpensAt))))))

(event EventBeginPlay
  (CallFunction|EstablishIMC)
  (CallFunction|Widget))

(fn ConstructionScript)

(fn MantleCheck
  (bind _camera (Variables|Default|GetCamera))
  (bind _returnvalue (Transformation|GetWorldLocation _camera))
  (bind (_outhit _returnvalue_2) (Collision|LineTraceByChannel _returnvalue (+ _returnvalue (* (Math|Vector|GetForwardVector _camera) 4e+01)) "TraceTypeQuery1" false 0 "None")) ; Forward Trace
  (if _returnvalue_2
    (Variables|Default|SetbHitDetected true)
    (bind _returnvalue_3 (Collision|SphereTraceByChannel (+ (+ (.Location (Collision|BreakHitResult _outhit)) (* (Math|Vector|GetForwardVector (Variables|Default|GetCamera)) 7.5)) "0.000000,0.000000,40.000000") (+ (+ (+ (.Location (Collision|BreakHitResult _outhit)) (* (Math|Vector|GetForwardVector (Variables|Default|GetCamera)) 7.5)) "0.000000,0.000000,40.000000") "0.000000,0.000000,25.000000") 15.0 "TraceTypeQuery1" false 0 "None"))
    (if _returnvalue_3
      (Variables|Default|SetbHitDetected false)
      (else
        (Variables|Default|SetVector (+ (+ (.Location (Collision|BreakHitResult _outhit)) (* (Math|Vector|GetForwardVector (Variables|Default|GetCamera)) 7.5)) "0.000000,0.000000,40.000000"))))
    (return)))

(fn StartTiming
  (params (InConfig :type Struct%20Timing%20Config%20Structure))
  (if (< (Utilities|Time|GetGameTimeinSeconds) (Variables|Default|GetCooldownEndsAt))
    (return)
    (else
      (bind _output_get (Variables|Default|SetConfig InConfig))
      (bind _output_get_2 (Variables|Default|SetWindowOpensAt (+ (.opendelay _output_get) (Utilities|Time|GetGameTimeinSeconds))))
      (Variables|Default|SetWindowClosesAt (+ _output_get_2 (.windowlength _output_get)))
      (LocalVariables|SetMid (* (+ (Variables|Default|GetWindowOpensAt) (Variables|Default|GetWindowClosesAt)) 0.5))
      (bind _output_get_3 (LocalVariables|SetHalfPerfect (* (* (.windowlength _output_get) (.perfectpct _output_get)) 0.5)))
      (Variables|Default|SetPerfectStart (- (LocalVariables|GetMid) _output_get_3))
      (Variables|Default|SetPerfectEnd (+ (LocalVariables|GetMid) _output_get_3))
      (Variables|Default|SetbInTimingMode true)
      (CallFunction|Timer)
      (if (Utilities|IsValid (Variables|Default|GetTimingWidget))
        (Widget|SetVisibility (Variables|Default|GetTimingWidget) "Visible")
        (Variables|Default|SetbShowTimingUI true)))))

(fn ResolveTiming
  (params (PressedAt :type Float%20%28double-precision%29))
  (bind _config (Variables|Default|GetConfig))
  (Variables|Default|SetPressedAt PressedAt)
  (if (Variables|Default|GetbInTimingMode)
    (if (< (+ PressedAt (.earlylockout _config)) (Variables|Default|GetWindowOpensAt))
      (CallFunction|EndTiming false)
      (CallFunction|ApplyTimingResult "NewEnumerator5")
      (elif (< PressedAt (- (Variables|Default|GetWindowOpensAt) (.earlylockout _config)))
        (CallFunction|EndTiming false)
        (CallFunction|ApplyTimingResult "NewEnumerator1")
        (elif (< PressedAt (Variables|Default|GetWindowOpensAt))
          (CallFunction|EndTiming false)
          (CallFunction|ApplyTimingResult "NewEnumerator5")
          (elif (<= (Variables|Default|GetPressedAt) (Variables|Default|GetWindowClosesAt))
            (if (and (>= (Variables|Default|GetPressedAt) (Variables|Default|GetPerfectStart)) (<= (Variables|Default|GetPressedAt) (Variables|Default|GetPerfectEnd)))
              (CallFunction|EndTiming false)
              (CallFunction|ApplyTimingResult "NewEnumerator3")
              (else
                (CallFunction|EndTiming false)
                (CallFunction|ApplyTimingResult "NewEnumerator2")))
            (elif (<= (Variables|Default|GetPressedAt) (+ (.lategrace (Variables|Default|GetConfig)) (Variables|Default|GetWindowClosesAt)))
              (CallFunction|EndTiming false)
              (CallFunction|ApplyTimingResult "NewEnumerator5")
              (else
                (CallFunction|EndTiming false)
                (CallFunction|ApplyTimingResult "NewEnumerator5")))))))))

(fn ApplyTimingResult
  (params (Result :type E_AttackTimingResult%20Enum :default "NewEnumerator1"))
  (switch Utilities|FlowControl|Switch|SwitchonE_AttackTimingResult Result
    (:NewEnumerator1
      (Development|PrintString "Early" true true "(R=0.883050,G=0.032194,B=1.000000,A=1.000000)"))
    (:NewEnumerator2
      (Development|PrintString "Good" true true "(R=1.000000,G=0.987267,B=0.000000,A=1.000000)"))
    (:NewEnumerator3
      (Development|PrintString "Perfect" true true "(R=0.090696,G=1.000000,B=0.000000,A=1.000000)"))
    (:NewEnumerator5
      (Development|PrintString "Miss" true true "(R=1.000000,G=0.023545,B=0.000000,A=1.000000)"))))

(fn EndTiming
  (params (MissIfUnresolved :type Boolean))
  (if (and MissIfUnresolved (Variables|Default|GetbInTimingMode))
    (CallFunction|ApplyTimingResult "NewEnumerator5")
    (Variables|Default|SetbInTimingMode false)
    (Variables|Default|SetCooldownEndsAt (+ (Utilities|Time|GetGameTimeinSeconds) (.cooldown (Variables|Default|GetConfig))))
    (Widget|SetVisibility (Variables|Default|GetTimingWidget) "Hidden")
    (Variables|Default|SetbShowTimingUI false)))