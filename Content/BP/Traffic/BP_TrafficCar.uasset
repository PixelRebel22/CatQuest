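; BP_TrafficCar is a traffic car that drives in a straight line and kills the player on contact.
; BeginPlay records its start position and forward direction, and Tick moves it along that direction at Speed with a swept offset.
; The car destroys itself once it has travelled RoadLength from its start.
; Its Box overlap casts the other actor to BP_PlayerCopy and calls KillPlayer.
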(event OnComponentBeginOverlap(Box)
  (params (OverlappedComponent :type Primitive%20Component%20Object%20Reference) (OtherActor :type Actor%20Object%20Reference) (OtherComp :type Primitive%20Component%20Object%20Reference) (OtherBodyIndex :type Integer) (bFromSweep :type Boolean) (SweepResult :type Hit%20Result%20Structure%20%28by%20ref%29))
  (bind _asbp_player_copy (Utilities|Casting|CastToBP_PlayerCopy OtherActor))
  (Default|KillPlayer _asbp_player_copy _asbp_player_copy))

(event EventBeginPlay
  (Variables|Default|SetStartTransform (Transformation|GetActorTransform))
  (Variables|Default|SetStartLocation (Transformation|GetActorLocation))
  (Variables|Default|SetMoveDir (Math|Vector|Normalize (Transformation|GetActorForwardVector))))

(event EventTick
  (params (DeltaSeconds :type Float%20%28single-precision%29))
  (Transformation|AddActorWorldOffset (* (* (Variables|Default|GetSpeed) DeltaSeconds) (Variables|Default|GetMoveDir)) true)
  (if (>= (Math|Vector|Distance(Vector) (Transformation|GetActorLocation) (Variables|Default|GetStartLocation)) (Variables|Default|GetRoadLength))
    (Variables|Default|SetbReachedEnd true)
    (Actor|DestroyActor)))

(fn ConstructionScript)