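; BP_TrafficLane is a traffic lane that spawns one car at a time at its spawn point, starting at BeginPlay.
; A positive road length override is copied to the spawned car, and only then is its destroyed event bound.
; When a bound car is destroyed, the lane waits out the respawn delay and spawns a replacement.
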(event Custom|SpawnCar
  (Variables|Default|SetbIsSpawning true)
  (bind _returnvalue (Game|SpawnActorfromClass (Variables|Default|GetCarClass) (Transformation|GetActorTransform (Variables|Default|GetSpawnPoint)) "Undefined" "MultiplyWithRoot" 0 0))
  (bind _output_get (Variables|Default|SetCurrentCar _returnvalue))
  (if (> (Variables|Default|GetOverrideRoadLength) 0.0)
    (Variables|/Game/BP/Traffic/BP_TrafficCar.BP_TrafficCar_C|SetRoadLength _output_get (Variables|Default|GetOverrideRoadLength))
    (Game|BindEventtoOnDestroyed _output_get (delegate Custom|OnCarDestroyed))))

(event Custom|OnCarDestroyed
  (params (DestroyedActor :type Actor%20Object%20Reference))
  (Variables|Default|SetCurrentCar 0)
  (Utilities|FlowControl|Delay (Variables|Default|GetRespawnDelay))
  (CallFunction|SpawnCar))

(event EventBeginPlay
  (if (not (Variables|Default|GetbIsSpawning))
    (CallFunction|SpawnCar)))

(fn ConstructionScript)